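; Blueprint actor that plays a level sequence in response to a Solaris boss event, named for the boss kill.
; On BeginPlay it registers itself as a listener with the GodfallGameState event manager, and unregisters on EndPlay.
; When an event arrives from a CSolaris notifier, it plays the referenced LevelSequenceActor's sequence, without checking which event type was sent.
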(event `self.ReceiveBeginPlay`
  (bind _asgodfall_game_state (cast `GodfallGameState` (`GameplayStatics.GetGameState`)))
  (`EventManagerComponent.RegistListener` (`GodfallGameState.GetEventManager` _asgodfall_game_state) self))

(event `self.ReceiveEndPlay`
  (params (EndPlayReason :type "EEndPlayReason Enum" :default "Destroyed"))
  (bind _asgodfall_game_state (cast `GodfallGameState` (`GameplayStatics.GetGameState`)))
  (`EventManagerComponent.UnregistListener` (`GodfallGameState.GetEventManager` _asgodfall_game_state) self))

(event `EventListenerInterface.OnEventListen`
  (params (Notifier :type "Object Object Reference") (Name :type "Name (by ref)") (Tag :type "Name (by ref)"))
  (cast `CSolaris` Notifier)
  (`MovieSceneSequencePlayer.Play` (`LevelSequenceActor.SequencePlayer` (`self.Level Sequence Actor`))))

(fn `UserConstructionScript`)