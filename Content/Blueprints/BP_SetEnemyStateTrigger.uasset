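; BP_SetEnemyStateTrigger is a trigger actor that changes the state of a set of enemies when the player enters it.
; On overlap with an actor tagged Player, it loops over its Enemies array and skips invalid entries.
; Each remaining enemy gets the trigger's RunAI value written to MRunAI and is shown or hidden according to Visible.
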(event `self.ReceiveActorBeginOverlap`
  (params (OtherActor :type "Actor Object Reference"))
  (if (`self.ActorHasTag` OtherActor "Player")
    (for _array_element (`self.Enemies`)
      (`/Engine/EditorBlueprintResources/StandardMacros.IsValid` _array_element
        (:`Is Valid`
          (`|ExecutionSequence`
            (:`then_0`
              (set `GodfallEnemyBase.mRunAI` (`self.RunAI`) _array_element))
            (:`then_1`
              (`self.SetActorHiddenInGame` _array_element (not (`self.Visible`))))))))))

(fn `UserConstructionScript`)