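; Sungate door actor with three panels that slide apart left, right and up when the player approaches from its back side.
; While the Trigger is overlapped, Tick checks for Player-tagged Characters and uses a forward-vector dot product to allow one-sided opening; ending overlap closes it.
; Tick interpolates panels by DoorState until within a distance limit.
; Door events restart audio on movement and snap panels to final positions.
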(event `self.ReceiveBeginPlay`)

(event `self.ReceiveTick`
  (params (DeltaSeconds :type "Float (single-precision)"))
  (bind _leftdoor (`self.LeftDoor`))
  (bind _rightdoor (`self.RightDoor`))
  (bind _topdoor (`self.TopDoor`))
  (bind _leftdoor_2 (`self.LeftDoor`))
  (bind _rightdoor_2 (`self.RightDoor`))
  (bind _topdoor_2 (`self.TopDoor`))
  (bind _trigger (`self.Trigger`))
  (set `self.Delta Seconds` DeltaSeconds)
  (`|ExecutionSequence`
    (:`then_0`
      (if (`self.IsOverlappingTarget`)
        (bind _outactors (`KismetSystemLibrary.ComponentOverlapActors` _trigger (`SceneComponent.K2_GetComponentToWorld` _trigger) (`|MakeArray` "ObjectTypeQuery3" :!type "EObjectTypeQuery Enum") "/Script/Engine.Character"))
        (for _array_element _outactors
          (if (and (`self.ActorHasTag` _array_element "Player") (> (`KismetMathLibrary.Dot_VectorVector` (`KismetMathLibrary.Normal` (- (`self.K2_GetActorLocation` self) (`self.K2_GetActorLocation` _array_element))) (`self.GetActorForwardVector` self)) 0.0))
            (`self.OpenImplementation`)))))
    (:`then_1`
      (switch `EDoorState` (`self.DoorState`)
        (:`Opening`
          (`SceneComponent.K2_SetRelativeLocation` _leftdoor_2 (`KismetMathLibrary.VInterpTo` (`SceneComponent.RelativeLocation` _leftdoor_2) (`KismetMathLibrary.MakeVector` 0.0 (* (`self.HorizonOpenLength`) -1.0)) (`self.Delta Seconds`) (`self.OpenInterpSpeed`)) false false)
          (`SceneComponent.K2_SetRelativeLocation` _rightdoor_2 (`KismetMathLibrary.VInterpTo` (`SceneComponent.RelativeLocation` _rightdoor_2) (`KismetMathLibrary.MakeVector` 0.0 (`self.HorizonOpenLength`)) (`self.Delta Seconds`) (`self.OpenInterpSpeed`)) false false)
          (`SceneComponent.K2_SetRelativeLocation` _topdoor_2 (`KismetMathLibrary.VInterpTo` (`SceneComponent.RelativeLocation` _topdoor_2) (`KismetMathLibrary.MakeVector` 0.0 0.0 (`self.VerticalOpenLength`)) (`self.Delta Seconds`) (`self.OpenInterpSpeed`)) false false)
          (if (< (`KismetMathLibrary.Vector_Distance` (`SceneComponent.RelativeLocation` (`self.TopDoor`)) (`KismetMathLibrary.MakeVector` 0.0 0.0 (`self.VerticalOpenLength`))) (`self.OpenLimitDistance`))
            (`self.SetToOpen`)))
        (:`Closing`
          (`SceneComponent.K2_SetRelativeLocation` _leftdoor (`KismetMathLibrary.VInterpTo` (`SceneComponent.RelativeLocation` _leftdoor) (`KismetMathLibrary.MakeVector` 0.0) (`self.Delta Seconds`) (`self.CloseInterpSpeed`)) false false)
          (`SceneComponent.K2_SetRelativeLocation` _rightdoor (`KismetMathLibrary.VInterpTo` (`SceneComponent.RelativeLocation` _rightdoor) (`KismetMathLibrary.MakeVector` 0.0) (`self.Delta Seconds`) (`self.CloseInterpSpeed`)) false false)
          (`SceneComponent.K2_SetRelativeLocation` _topdoor (`KismetMathLibrary.VInterpTo` (`SceneComponent.RelativeLocation` _topdoor) (`KismetMathLibrary.MakeVector` 0.0) (`self.Delta Seconds`) (`self.CloseInterpSpeed`)) false false)
          (if (< (`KismetMathLibrary.Vector_Distance` (`SceneComponent.RelativeLocation` (`self.TopDoor`)) (`KismetMathLibrary.MakeVector` 0.0)) (`self.CloseLimitDistance`))
            (`self.SetToClose`)))))))

(event `self.DoorBeginOpen`
  (`|ExecutionSequence` :!label _label
    (:`then_0`
      (`AudioComponent.Stop` (`self.Audio`)))
    (:`then_1`
      (`AudioComponent.Play` (`self.Audio`) 0.0))))

(event `self.DoorBeginClose`
  (goto _label))

(event `self.OnOpenDirect`
  (`SceneComponent.K2_SetRelativeLocation` (`self.LeftDoor`) (`KismetMathLibrary.MakeVector` 0.0 (* (`self.HorizonOpenLength`) -1.0)) false false :!label _label_2)
  (`SceneComponent.K2_SetRelativeLocation` (`self.RightDoor`) (`KismetMathLibrary.MakeVector` 0.0 (`self.HorizonOpenLength`)) false false)
  (`SceneComponent.K2_SetRelativeLocation` (`self.TopDoor`) (`KismetMathLibrary.MakeVector` 0.0 0.0 (`self.VerticalOpenLength`)) false false))

(event `self.OnOpen`
  (goto _label_2))

(event `self.OnCloseDirect`
  (`SceneComponent.K2_SetRelativeLocation` (`self.LeftDoor`) (0.0 0.0 0.0) false false :!label _label_3)
  (`SceneComponent.K2_SetRelativeLocation` (`self.RightDoor`) (0.0 0.0 0.0) false false)
  (`SceneComponent.K2_SetRelativeLocation` (`self.TopDoor`) (0.0 0.0 0.0) false false))

(event `self.OnClose`
  (goto _label_3))

(event `self.Trigger.OnComponentBeginOverlap`
  (params (OverlappedComponent :type "PrimitiveComponent Object Reference") (OtherActor :type "Actor Object Reference") (OtherComp :type "PrimitiveComponent Object Reference") (OtherBodyIndex :type Integer) (bFromSweep :type Boolean) (SweepResult :type "HitResult Structure (by ref)"))
  (set `self.IsOverlappingTarget` true))

(event `self.Trigger.OnComponentEndOverlap`
  (params (OverlappedComponent :type "PrimitiveComponent Object Reference") (OtherActor :type "Actor Object Reference") (OtherComp :type "PrimitiveComponent Object Reference") (OtherBodyIndex :type Integer))
  (set `self.IsOverlappingTarget` false)
  (`self.CloseImplementation`))

(fn `UserConstructionScript`)