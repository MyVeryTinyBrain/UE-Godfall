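; BP_PlaySequenceTrigger is a trigger actor that plays a level sequence when an actor tagged Player overlaps it.
; The overlap event calls Play on the referenced LevelSequenceActor's player, with no guard against retriggering.
; If the SkipSeqeunce flag is set, it then gathers every LevelSequenceActor in the world and sends each to its end and stops it, including the one just started.
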(event `self.ReceiveActorBeginOverlap`
  (params (OtherActor :type "Actor Object Reference"))
  (if (`self.ActorHasTag` OtherActor "Player")
    (`MovieSceneSequencePlayer.Play` (`LevelSequenceActor.SequencePlayer` (`self.Level Sequence Actor`)))
    (if (`self.Skip Seqeunce`)
      (bind _outactors (`GameplayStatics.GetAllActorsOfClass` "/Script/LevelSequence.LevelSequenceActor"))
      (if (`KismetArrayLibrary.Array_IsNotEmpty` _outactors)
        (for _array_element _outactors
          (`MovieSceneSequencePlayer.GoToEndAndStop` (`LevelSequenceActor.SequencePlayer` _array_element)))))))

(fn `UserConstructionScript`)